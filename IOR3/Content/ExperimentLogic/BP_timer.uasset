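; BP_timer runs a spatial cueing reaction-time trial with a fixation object and left and right cubes.
; startTrial_Event enables input and randomizes cue side, target side and stimulus onset asynchrony.
; Space starts a delay-timed sequence of fixation, brief cue and target by swapping materials, then timestamps target onset and calls OnFinish.
; Left mouse click prints reaction time since that timestamp, without checking side.
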(event `startTrial_Event`
  ; Get Character Input
  (`self.EnableInput` (`GameplayStatics.GetPlayerController` 0))
  (`KismetMaterialLibrary.CreateDynamicMaterialInstance` "/Game/ExperimentLogic/cueTarget.cueTarget" (`self.dynMesh`))
  ; Conditions
  ;; Set Sides; 0 = left 1 = right
  (set `self.cueSide` (`KismetMathLibrary.RandomIntegerInRange` 0 1))
  (set `self.targetSide` (`KismetMathLibrary.RandomIntegerInRange` 0 1))
  ;; Set SOA
  (set `self.targetDelay` (/ (`|GetArrayItem` (`self.SOAset`) (`KismetMathLibrary.RandomIntegerInRange` 0 3)) 1000.0)))

(event `Key|SpaceBar`
  (params (Key :type "Key Structure"))
  (:`Pressed`
    (`PrimitiveComponent.CreateDynamicMaterialInstance` (`self.fixation`) 0 "/Game/ExperimentLogic/cueTarget.cueTarget" "None")
    (`KismetSystemLibrary.Delay` 0.5)
    (`PrimitiveComponent.CreateDynamicMaterialInstance` (`self.fixation`) 0 "/Game/LevelPrototyping/Materials/M_Solid.M_Solid" "None")
    ; Cue
    (if (`KismetMathLibrary.Conv_IntToBool` (`self.cueSide`))
      (`PrimitiveComponent.CreateDynamicMaterialInstance` (`self.rightCube`) 0 "/Game/ExperimentLogic/cueTarget.cueTarget" "None")
      ; Fixation
      (`KismetSystemLibrary.Delay` 0.1)
      (`PrimitiveComponent.CreateDynamicMaterialInstance` (`self.rightCube`) 0 "/Game/LevelPrototyping/Materials/M_Solid.M_Solid" "None")
      (else
        (`PrimitiveComponent.CreateDynamicMaterialInstance` (`self.LeftCube`) 0 "/Game/ExperimentLogic/cueTarget.cueTarget" "None")
        (`KismetSystemLibrary.Delay` 0.1)
        (`PrimitiveComponent.CreateDynamicMaterialInstance` (`self.LeftCube`) 0 "/Game/LevelPrototyping/Materials/M_Solid.M_Solid" "None")))
    (`PrimitiveComponent.CreateDynamicMaterialInstance` (`self.fixation`) 0 "/Game/ExperimentLogic/cueTarget.cueTarget" "None")
    ; SOA
    (`KismetSystemLibrary.Delay` (`self.targetDelay`))
    ; Target
    (`PrimitiveComponent.CreateDynamicMaterialInstance` (`self.fixation`) 0 "/Game/LevelPrototyping/Materials/M_Solid.M_Solid" "None")
    (bind _output_get (set `self.startTime` (`KismetSystemLibrary.GetGameTimeInSeconds`)))
    (if (`KismetMathLibrary.Conv_IntToBool` (`self.targetSide`))
      (`PrimitiveComponent.CreateDynamicMaterialInstance` (`self.rightCube`) 0 "/Game/ExperimentLogic/cueTarget.cueTarget" "None")
      (else
        (`PrimitiveComponent.CreateDynamicMaterialInstance` (`self.LeftCube`) 0 "/Game/ExperimentLogic/cueTarget.cueTarget" "None")))
    (`self.onFinish`)))

(event `Key|LeftMouseButton`
  (params (Key :type "Key Structure"))
  (:`Pressed`
    (bind _output_get (set `self.endTime` (`KismetSystemLibrary.GetGameTimeInSeconds`)))
    (bind _output_get_2 (set `self.RT` (- _output_get (stale `Key|SpaceBar` _output_get))))
    (`KismetSystemLibrary.PrintString` (`KismetStringLibrary.Conv_DoubleToString` _output_get_2))))

(fn `UserConstructionScript`)