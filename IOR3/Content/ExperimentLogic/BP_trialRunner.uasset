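; Trial runner Blueprint that advances trials within an experiment block.
; On BeginPlay it binds a handler to the OnFinish event of the referenced experiment.
; Each finish increments NumberTrial, then starts another trial if it exceeds CountTrial, otherwise prints that the block is finished.
; A one-second timer is set before StartTrial with no event connected, and the first trial is not started here.
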(event `self.ReceiveBeginPlay`
  (add `/Game/ExperimentLogic/BP_timer.onFinish` (`self.expRef`) (delegate `HandleTrialFinished`)))

(event `HandleTrialFinished`
  ; Add 1 to trial and check if current trial number matches max number of trials before next block
  (set `self.numberTrial` (+ (`self.numberTrial`) 1))
  ; countTrial < numberTrial
  (if (> (`self.numberTrial`) (`self.countTrial`))
    (`KismetSystemLibrary.K2_SetTimerDelegate` :`Time` 1.0)
    (`/Game/ExperimentLogic/BP_timer.startTrial` (`self.expRef`))
    (else
      (`KismetSystemLibrary.PrintString` "Block Finished"))))

(fn `BP_trialRunner_AutoGenFunc`
  (params (NewParam :type Boolean)))

(fn `UserConstructionScript`)